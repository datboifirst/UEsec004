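; Adv_Platform_BP is a platform that a MyCharacter can drop through by toggling the collision of its RenderComponent.
; Overlapping UpperBox turns collision on, while overlapping LowerBox enables player input on the platform.
; Pressing C turns collision off, with a CollisionStatus flag gating the toggles.
; A custom overlap-style event, with no binding shown, re-enables collision after a short delay but clears the flag.
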(event `self.UpperBox.OnComponentBeginOverlap`
  (params (OverlappedComponent :type "PrimitiveComponent Object Reference") (OtherActor :type "Actor Object Reference") (OtherComp :type "PrimitiveComponent Object Reference") (OtherBodyIndex :type Integer) (bFromSweep :type Boolean) (SweepResult :type "HitResult Structure (by ref)"))
  ;[1 1 1] Upper Collision
  (cast `/Game/Blueprint/MyCharacter` OtherActor)
  (if (not (`self.Collision Status`))
    (`PrimitiveComponent.SetCollisionEnabled` (`self.RenderComponent`) "QueryAndPhysics")
    (set `self.Collision Status` true)))

(event `self.LowerBox.OnComponentBeginOverlap`
  (params (OverlappedComponent :type "PrimitiveComponent Object Reference") (OtherActor :type "Actor Object Reference") (OtherComp :type "PrimitiveComponent Object Reference") (OtherBodyIndex :type Integer) (bFromSweep :type Boolean) (SweepResult :type "HitResult Structure (by ref)"))
  ;[1 1 1] Lower Collision
  (cast `/Game/Blueprint/MyCharacter` OtherActor)
  (`self.EnableInput` (`GameplayStatics.GetPlayerController` 0))
  (`KismetSystemLibrary.PrintString` "Hello"))

(event `Key|C`
  (params (Key :type "Key Structure"))
  ;[1 1 1] Press C to jump down
  (:`Pressed`
    (`KismetSystemLibrary.PrintString` "jump down")
    (if (`self.Collision Status`)
      (`PrimitiveComponent.SetCollisionEnabled` (`self.RenderComponent`) "NoCollision")
      (set `self.Collision Status` false))))

(event `CustomEvent`
  (params (OverlappedComponent :type "PrimitiveComponent Object Reference") (OtherActor :type "Actor Object Reference") (OtherComp :type "PrimitiveComponent Object Reference") (OtherBodyIndex :type Integer) (bFromSweep :type Boolean) (SweepResult :type "HitResult Structure (by ref)"))
  ;[1 1 1] Fixed Bug
  (cast `/Game/Blueprint/MyCharacter` OtherActor)
  (if (`self.Collision Status`)
    (`KismetSystemLibrary.Delay` 0.5)
    (`PrimitiveComponent.SetCollisionEnabled` (`self.RenderComponent`) "QueryAndPhysics")
    (set `self.Collision Status` false)))

(fn `UserConstructionScript`)