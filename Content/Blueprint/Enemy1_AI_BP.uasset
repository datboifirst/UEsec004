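; Paper2D enemy character that patrols back and forth on its own, using walk and idle flipbooks.
; Each Tick adds forward movement input, sets IsMovingRight from X velocity and picks the flipbook from falling state and speed.
; A one-second Delay on Tick serves as a repeating timer that rotates the actor 180 degrees to reverse its path, with no sensing involved.
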(event `UpdateAnimation`
  (bind _paperflipbook (`self.PaperFlipbook`))
  (if (`NavMovementComponent.IsFalling` (`self.CharacterMovement`))
    (`PaperFlipbookComponent.SetFlipbook` _paperflipbook "/Game/Asset3_Flipbooks/Enemy_Walk.Enemy_Walk")
    (else
      (`PaperFlipbookComponent.SetFlipbook` _paperflipbook (select `bool` (> (`KismetMathLibrary.VSize` (`self.GetVelocity`)) 0.0) :`false` "/Game/Asset3_Flipbooks/Enemy_Idle.Enemy_Idle" :`true` "/Game/Asset3_Flipbooks/Enemy_Walk.Enemy_Walk" :!type "PaperFlipbook Object Reference")))))

(event `Check Direction`
  (bind _returnvalue_x (`KismetMathLibrary.BreakVector` (`self.GetVelocity`)))
  (bind _returnvalue_x_2 (`KismetMathLibrary.BreakVector` (`self.GetVelocity`)))
  (if (> _returnvalue_x_2 0.0)
    (set `self.IsMovingRight` true)
    (elif (< _returnvalue_x 0.0)
      (set `self.IsMovingRight` false))))

(event `Movement`
  (`self.AddMovementInput` (`self.GetActorForwardVector`)))

(event `Turn Char`
  (`self.K2_SetActorRotation` (`KismetMathLibrary.ComposeRotators` (`self.K2_GetActorRotation`) (struct :`Yaw` 180.0))))

(event `self.ReceiveTick`
  (params (DeltaSeconds :type "Float (single-precision)"))
  (`|ExecutionSequence`
    (:`then_0`
      (`self.Movement`)
      (`self.Check Direction`)
      (`self.UpdateAnimation`))
    (:`then_1`
      (`KismetSystemLibrary.Delay` 1.0)
      (`self.Turn Char`))))

(fn `UserConstructionScript`)