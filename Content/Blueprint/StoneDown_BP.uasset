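; StoneDown_BP is a falling stone object using Super Mario Bros. 3 sprites that repeats a drop motion on its own.
; After a short BeginPlay delay, a timeline lerps the PaperSprite's relative location between points A and B.
; Each update also swaps the stone's face sprite once the timeline's Speed track reaches a threshold.
; When the timeline finishes, DropStone waits briefly and calls itself again, looping indefinitely.
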(event `self.ReceiveBeginPlay`
  ;[1 1 1] Start
  (`KismetSystemLibrary.Delay` 0.5)
  ;;[0.2602 0.8801 1] Call drop stone event
  (`self.Drop Stone`))

(event `Drop Stone`
  ;[0.4635 1 0.5216] DropStone Script
  (bind (_direction _speed) (`Timeline|Timeline_Animation` :!via `PlayFromStart`)
    (:`Update`
      (`|ExecutionSequence`
        (:`then_0`
          (`SceneComponent.K2_SetRelativeLocation` (`self.PaperSprite`) (`KismetMathLibrary.VLerp` (`self.A`) (`self.B`) _speed) false false))
        (:`then_1`
          (`self.Changing Faces `))))
    (:`Finished`
      (`KismetSystemLibrary.Delay` 1.0)
      ;;[0.06771 0.95 1] Call drop stone again
      (`self.Drop Stone`))))

(event `Changing Faces`
  (bind _papersprite (`self.PaperSprite`))
  ;[0.5854 0.153 0.7344] Changing Faces
  (if (>= (stale `Drop Stone` _speed) 0.8)
    (`PaperSpriteComponent.SetSprite` _papersprite "/Game/Asset2_Mario/SMB3_Objects_Sprite_388.SMB3_Objects_Sprite_388")
    (else
      (`PaperSpriteComponent.SetSprite` _papersprite "/Game/Asset2_Mario/SMB3_Objects_Sprite_371.SMB3_Objects_Sprite_371"))))

(fn `NewFunction`)

(fn `UserConstructionScript`)